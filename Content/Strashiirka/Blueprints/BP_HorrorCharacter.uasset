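; Player character Blueprint for a horror game that collects items on contact and handles touch controls.
; On BeginPlay it switches to game-only input and hides the mouse cursor.
; Overlapped actors implementing BPI_Collectables receive a Collect call.
; Touch thumbstick events feed DoMove and DoAim, while the touch jump button is repurposed to start and end sprinting.
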(event Collision|EventActorBeginOverlap
  (params (OtherActor :type Actor%20Object%20Reference))
  (bind _asbpi_collectables (Utilities|Casting|CastToBPI_Collectables OtherActor))
  (Default|Collect _asbpi_collectables))

(event EventBeginPlay
  (bind _returnvalue (Game|GetPlayerController 0))
  (Input|SetInputModeGameOnly _returnvalue false)
  (Variables|/Script/Engine.PlayerController|SetbShowMouseCursor _returnvalue false))

(event EventPrimaryThumbstick
  (params (Axis :type Vector%202D%20Structure))
  ;[1 1 1] Touch Inputs for Horror Character
  (Class|StrashiirkaCharacter|DoMove (.x Axis) (.y Axis)))

(event EventTouchJumpStart
  ;[1 1 1] Touch Inputs for Horror Character
  (Class|HorrorCharacter|DoStartSprint))

(event EventTouchJumpEnd
  ;[1 1 1] Touch Inputs for Horror Character
  (Class|HorrorCharacter|DoEndSprint))

(event EventSecondaryThumbstick
  (params (Axis :type Vector%202D%20Structure))
  ;[1 1 1] Touch Inputs for Horror Character
  (Class|StrashiirkaCharacter|DoAim (.x Axis) (.y Axis)))

(fn ConstructionScript)
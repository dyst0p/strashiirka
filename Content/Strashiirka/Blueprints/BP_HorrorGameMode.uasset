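; BP_HorrorGameMode is the horror game's game mode, tracking sheet collection and deciding win or game over.
; On BeginPlay it counts all BP_Sheet actors as the total and broadcasts progress through OnSheetsUpdated.
; AddSheetCollected increments and rebroadcasts the count, calling Win when it matches the total.
; Win and GameOver fire their dispatchers, then EndGame pauses the game and shows the UI_EndGamePanel widget.
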(event EventBeginPlay
  (bind _outactors (Actor|GetAllActorsOfClass "/Game/Strashiirka/Blueprints/BP_Sheet.BP_Sheet_C"))
  (bind _output_get (Variables|Default|SetTotalSheets (Utilities|Array|Length _outactors)))
  (Default|CallOnSheetsUpdated (Variables|Default|GetCollectedSheets) _output_get))

(event EventTick
  (params (DeltaSeconds :type Float%20%28single-precision%29)))

(fn ConstructionScript)

(fn AddSheetCollected
  (bind _totalsheets (Variables|Default|GetTotalSheets))
  (bind _result (Math|Integer|IncrementInt (Variables|Default|GetCollectedSheets))
    (:%20%20
      (Default|CallOnSheetsUpdated _result _totalsheets)
      (if (== _result _totalsheets)
        (CallFunction|Win)))))

(fn GameOver
  (Development|PrintString "Game Over")
  (Default|CallOnGameOver)
  (CallFunction|EndGame))

(fn Win
  (Development|PrintString "You Win!")
  (Variables|Default|SetIsWin true)
  (Default|CallOnWin)
  (CallFunction|EndGame))

(fn GetIsWin
  (return (Variables|Default|GetIsWin)))

(fn EndGame
  (Game|SetGamePaused true)
  (bind _returnvalue (UserInterface|CreateWidget "/Game/Strashiirka/UI/UI_EndGamePanel.UI_EndGamePanel_C" (Game|GetPlayerController 0)))
  (UserInterface|Viewport|AddtoViewport _returnvalue 0))
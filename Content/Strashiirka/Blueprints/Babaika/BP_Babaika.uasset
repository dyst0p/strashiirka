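; BP_Babaika is a monster pawn that relentlessly chases the player in a horror game.
; Each tick it feeds movement input straight toward the player's location, with no pathfinding.
; It listens to the horror game mode's sheet updates and scales its floating movement speed by the fraction of sheets collected, also printing that value.
; Overlapping the player triggers the game mode's GameOver.
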(event Custom|Update%20Speed
  (params (Collected :type Integer) (Total :type Integer))
  (Development|PrintString (Utilities|String|ToString(Float) (/ (* Collected (Variables|Default|GetMaxSpeed)) Total)))
  (Variables|/Script/Engine.FloatingPawnMovement|SetMaxSpeed (Variables|Default|GetFloatingPawnMovement) (/ (* Collected (Variables|Default|GetMaxSpeed)) Total)))

(event EventBeginPlay
  (Variables|Default|SetPlayer (Game|Player|GetPlayerPawn 0))
  (bind _asbp_horror_game_mode (Utilities|Casting|CastToBP_HorrorGameMode (Game|GetGameMode)))
  (EventDispatchers|BindEventtoOnSheetsUpdated _asbp_horror_game_mode (delegate Custom|Update%20Speed)))

(event EventTick
  (params (DeltaSeconds :type Float%20%28single-precision%29))
  (Pawn|Input|AddMovementInput (Math|Vector|Normalize (- (Transformation|GetActorLocation (Variables|Default|GetPlayer)) (Transformation|GetActorLocation))) 1.0 false))

(event Collision|EventActorBeginOverlap
  (params (OtherActor :type Actor%20Object%20Reference))
  (if (== OtherActor (Variables|Default|GetPlayer))
    (bind _asbp_horror_game_mode (Utilities|Casting|CastToBP_HorrorGameMode (Game|GetGameMode)))
    (Default|GameOver _asbp_horror_game_mode)))

(fn ConstructionScript)